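; BP_Enemy2 is an enemy Blueprint for a robot character with a sword, exhausts and a child actor on its shield socket.
; Its construction script attaches both exhausts, the sword and the child actor to named sockets on the mesh.
; The PlayAttackAnim event casts the mesh's anim instance to ABP_Robot3 and forwards the call, leaving the attack animation to that Animation Blueprint.
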(event EventPlayAttackAnim
  (bind _asabp_robot_3 (Utilities|Casting|CastToABP_Robot3 (Components|SkeletalMesh|GetAnimInstance (Variables|Character|GetMesh))))
  (Default|PlayAttackAnim _asabp_robot_3))

(fn ConstructionScript
  (Class|SceneComponent|Attachto (Variables|Default|GetExhaust1) (Variables|Character|GetMesh) "Exhaust" "KeepRelativeOffset" true)
  (Class|SceneComponent|Attachto (Variables|Default|GetSword) (Variables|Character|GetMesh) "Sword" "KeepRelativeOffset" true)
  (Class|SceneComponent|Attachto (Variables|Default|GetChildActor) (Variables|Character|GetMesh) "Shield" "KeepRelativeOffset" true))