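; Fire rate pickup that raises the player character's ShotsPerSecond on overlap, then plays a pickup sound and destroys itself.
; The increase is inversely proportional to the current rate, so repeated pickups give diminishing returns.
; Tick bobs the actor with a sine of game time and spins it in yaw; the bob offset is applied per frame without delta-time scaling, unlike the spin.
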(event EventBeginPlay)

(event EventActorBeginOverlap
  (params (OtherActor :type Actor%20Object%20Reference))
  (bind _asbp_player_character (Utilities|Casting|CastToBP_PlayerCharacter OtherActor))
  (Variables|/Script/SecondPersonShooter.PlayerCharacter|SetShotsPerSecond _asbp_player_character (+ (Variables|/Script/SecondPersonShooter.PlayerCharacter|GetShotsPerSecond _asbp_player_character) (/ 2.0 (Variables|/Script/SecondPersonShooter.PlayerCharacter|GetShotsPerSecond _asbp_player_character))))
  (Audio|PlaySoundatLocation "/Game/Assets/Audio/ammo-pick-up.ammo-pick-up" (Transformation|GetActorLocation))
  (Actor|DestroyActor))

(event EventTick
  (params (DeltaSeconds :type Float%20%28single-precision%29))
  (bind _returnvalue (Transformation|GetActorLocation))
  (bind _returnvalue_2 (Transformation|GetActorRotation))
  (Transformation|SetActorLocation (Math|Vector|MakeVector (.x _returnvalue) (.y _returnvalue) (+ (.z _returnvalue) (* (Math|Trig|Sin(Radians) (* (Utilities|Time|GetGameTimeinSeconds) 1.0)) 0.2))) false false)
  (Transformation|SetActorRotation (Math|Rotator|MakeRotator (.roll _returnvalue_2) (.pitch _returnvalue_2) (+ (.yaw _returnvalue_2) (* (Utilities|Time|GetWorldDeltaSeconds) 8.0)))))

(fn ConstructionScript)