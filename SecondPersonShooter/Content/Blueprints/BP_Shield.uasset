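; BP_Shield is a shield actor with its own health that drops loose when destroyed.
; It binds to its any-damage event at BeginPlay and subtracts incoming damage from Health.
; At zero or below, the static mesh detaches, keeping its world position, and starts simulating physics.
; An unconnected graph that would drop the mesh when its attach parent is missing or its owner is dead never runs.
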(event Custom|OnTakeAnyDamage_Event
  (params (Damage :type Float%20%28single-precision%29) (DamageType :type Damage%20Type%20Object%20Reference) (InstigatedBy :type Controller%20Object%20Reference) (DamageCauser :type Actor%20Object%20Reference))
  (bind _output_get (Variables|Default|SetHealth (- (Variables|Default|GetHealth) Damage)))
  (if (<= _output_get 0.0)
    (Class|SceneComponent|DetachfromParent (Variables|Default|GetStaticMesh) true true)
    (Physics|SetSimulatePhysics (Variables|Default|GetStaticMesh) true)))

(event EventBeginPlay
  (EventDispatchers|AssignOnTakeAnyDamage (delegate Custom|OnTakeAnyDamage_Event)))

(event EventTick
  (params (DeltaSeconds :type Float%20%28single-precision%29)))

(fn ConstructionScript)