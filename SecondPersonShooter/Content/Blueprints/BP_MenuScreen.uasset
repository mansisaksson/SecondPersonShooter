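; BP_MenuScreen is a menu screen actor that drives map selection and game start by gamepad through its WB_MenuScreen widget.
; D-pad up and down step to the previous or next map, and the bottom face button starts the game.
; Each key event acts only while BP_GameMode reports gameplay is not running, then forwards the call to the user widget of its Widget component.
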(event EventBeginPlay)

(event Collision|EventActorBeginOverlap
  (params (OtherActor :type Actor%20Object%20Reference)))

(event EventTick
  (params (DeltaSeconds :type Float%20%28single-precision%29)))

(event Input|GamepadEvents|GamepadDPadUp
  (params (Key :type Key%20Structure :default "AnyKey"))
  (:Pressed
    (bind _asbp_game_mode (Utilities|Casting|CastToBP_GameMode (Game|GetGameMode)))
    (if (not (Class|DefaultGameMode|IsGameplayRunning _asbp_game_mode))
      (bind _aswb_menu_screen (Utilities|Casting|CastToWB_MenuScreen (UserInterface|GetUserWidgetObject (Variables|Default|GetWidget))))
      (Default|PrevMap _aswb_menu_screen))))

(event Input|GamepadEvents|GamepadDPadDown
  (params (Key :type Key%20Structure :default "AnyKey"))
  (:Pressed
    (bind _asbp_game_mode (Utilities|Casting|CastToBP_GameMode (Game|GetGameMode)))
    (if (not (Class|DefaultGameMode|IsGameplayRunning _asbp_game_mode))
      (bind _aswb_menu_screen (Utilities|Casting|CastToWB_MenuScreen (UserInterface|GetUserWidgetObject (Variables|Default|GetWidget))))
      (Default|NextMap _aswb_menu_screen))))

(event Input|GamepadEvents|GamepadFaceButtonBottom
  (params (Key :type Key%20Structure :default "AnyKey"))
  (:Pressed
    (bind _asbp_game_mode (Utilities|Casting|CastToBP_GameMode (Game|GetGameMode)))
    (if (not (Class|DefaultGameMode|IsGameplayRunning _asbp_game_mode))
      (bind _aswb_menu_screen (Utilities|Casting|CastToWB_MenuScreen (UserInterface|GetUserWidgetObject (Variables|Default|GetWidget))))
      (Default|StartGame _aswb_menu_screen))))

(fn ConstructionScript)