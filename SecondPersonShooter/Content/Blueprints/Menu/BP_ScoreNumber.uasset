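; BP_ScoreNumber is a floating world-space text actor that shows a "+" followed by its DamageValue.
; Construction sets the text and picks a randomly offset start location around the spawn point.
; On BeginPlay a timeline lifts the number from that location while fading its text alpha, then destroys the actor.
; Each tick yaws the text toward the player character's possessed enemy.
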(event EventBeginPlay
  (bind _timeline (Variables|Default|GetTimeline))
  (bind _startlocation (Variables|Default|GetStartlocation))
  (bind _textrender (Variables|Default|GetTextRender))
  (bind _textrendercolor (Variables|/Script/Engine.TextRenderComponent|GetTextRenderColor _textrender))
  ;[1 1 1] PositionDisplacement
  (bind _position (Timeline|Timeline PlayFromStart)
    (:Update
      (Transformation|SetActorLocation (Math|Vector|MakeVector (.x _startlocation) (.y _startlocation) (+ (.z _startlocation) (* _position 5e+01))) false false)
      ;[1 1 1] Alpha
      (Rendering|Components|TextRender|SetTextRenderColor _textrender (Math|Color|MakeColor (.b _textrendercolor) (.g _textrendercolor) (.r _textrendercolor) (Math|Conversions|ToByte(Integer) (Math|Float|Truncate (* 255 (- 1.0 (/ (Components|Timeline|GetPlaybackPosition _timeline) (Components|Timeline|GetTimelineLength _timeline)))))))))
    (:Finished
      (Actor|DestroyActor))))

(event EventTick
  (params (DeltaSeconds :type Float%20%28single-precision%29))
  (bind _asbp_player_character (Utilities|Casting|CastToBP_PlayerCharacter (Game|Player|GetPlayerPawn 0)))
  ;[1 1 1] LookatPlayerView
  (Transformation|SetWorldRotation (Variables|Default|GetTextRender) (Math|Rotator|MakeRotator 0.0 0.0 (.yaw (Math|Rotator|FindLookatRotation (Transformation|GetActorLocation) (Transformation|GetActorLocation (Class|PlayerCharacter|GetPossessedEnemy _asbp_player_character))))) false false))

(fn ConstructionScript
  (bind _returnvalue (Transformation|GetActorLocation))
  (bind _returnvalue_2 (Math|Random|RandomFloatinRange 0.0 1e+02))
  (bind _returnvalue_3 (Math|Random|RandomUnitVector))
  (bind _returnvalue_4 (* _returnvalue_3 _returnvalue_2))
  (Rendering|Components|TextRender|SetText (Variables|Default|GetTextRender) (Utilities|Text|ToText(String) (Utilities|String|Append "+" (Utilities|String|ToString(Integer) (Variables|Default|GetDamageValue)))))
  (Variables|Default|SetStartlocation (Math|Vector|MakeVector (+ (.x _returnvalue) (.x _returnvalue_4)) (+ (.y _returnvalue) (.y _returnvalue_4)) (+ (.z _returnvalue) (.z _returnvalue_4)))))