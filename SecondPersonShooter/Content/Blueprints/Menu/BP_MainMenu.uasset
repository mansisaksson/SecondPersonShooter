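; In-world main menu actor for a VR game, showing WB_MainMenu and a controls screen on widget components.
; Input actions navigate and select items, gated by BP_GameMode state, and reset HMD pose.
; Play calls SwapCloser on the player and hands input to it and all BP_LevelSelect actors; Controls swaps widgets; Exit quits.
; Tick uses random Delays to periodically flicker the PointLight between full and half intensity.
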(event EventBeginPlay
  (Variables|Default|SetDefaultIntesity (Variables|/Script/Engine.LightComponentBase|GetIntensity (Variables|Default|GetPointLight)))
  (Rendering|SetVisibility (Variables|Default|GetControllsWidget) false false))

(event EventTick
  (params (DeltaSeconds :type Float%20%28single-precision%29))
  (if (Variables|Default|GetBlink)
    (Utilities|FlowControl|Delay (Math|Random|RandomFloatinRange 0.01 0.1))
    (bind _output_get (Variables|Default|SetBlinkIndex (+ (Variables|Default|GetBlinkIndex) 1)))
    (Rendering|Components|Light|SetIntensity (Variables|Default|GetPointLight) (/ (Variables|Default|GetDefaultIntesity) (Math|Conversions|ToFloat(Integer) (+ (Math|Integer|%(Integer) _output_get 2) 1))))
    (if (== _output_get (Variables|Default|GetAmountOfBlinks))
      (Rendering|SetVisibility (Variables|Default|GetPointLight) true false)
      (Variables|Default|SetBlink false)
      (Variables|Default|SetBlinkIndex 0))
    (else
      (Utilities|FlowControl|Delay (Math|Random|RandomFloatinRange 3.5 15.0))
      (Variables|Default|SetBlink true))))

(event Input|ActionEvents|InputActionAccept
  (params (Key :type Key%20Structure :default "AnyKey"))
  ;[1 1 1] Select Element
  (:Pressed
    (bind _asbp_game_mode (Utilities|Casting|CastToBP_GameMode (Game|GetGameMode)))
    (if (not (or (Class|DefaultGameMode|IsGameplayRunning _asbp_game_mode) (Class|DefaultGameMode|IsGameLoaded _asbp_game_mode)))
      (bind _aswb_main_menu (Utilities|Casting|CastToWB_MainMenu (UserInterface|GetUserWidgetObject (Variables|Default|GetMainMenuWidget))))
      (bind _selecteditem (Default|GetSelectedItem _aswb_main_menu))
      (switch string _selecteditem
        (:Play
          ;;[1 1 1] Play Pressed
          (bind _asbp_game_mode_2 (Utilities|Casting|CastToBP_GameMode (Game|GetGameMode)))
          (Utilities|IsValid (Class|DefaultGameMode|GetPlayerRef _asbp_game_mode_2)
            (:Is%20Valid
              (Class|PlayerCharacter|SwapCloser (Class|DefaultGameMode|GetPlayerRef _asbp_game_mode_2))
              (Input|EnableInput (Class|DefaultGameMode|GetPlayerRef _asbp_game_mode_2) (Game|GetPlayerController 0))
              (CallFunction|Disable)
              (bind _outactors (Actor|GetAllActorsOfClass "/Game/Blueprints/Menu/BP_LevelSelect.BP_LevelSelect_C"))
              (for _array_element _outactors
                (Default|Enable _array_element)))))
        (:Controls
          ;;[1 1 1] Comment
          (Rendering|SetVisibility (Variables|Default|GetControllsWidget) true false)
          (Rendering|SetVisibility (Variables|Default|GetMainMenuWidget) false false))
        (:Exit
          (Development|ExecuteConsoleCommand "quit"))))))

(event Input|ActionEvents|InputActionMenuDown
  (params (Key :type Key%20Structure :default "AnyKey"))
  ;[1 1 1] Next Element
  (:Pressed
    (if (Rendering|IsVisible (Variables|Default|GetMainMenuWidget))
      (bind _asbp_game_mode (Utilities|Casting|CastToBP_GameMode (Game|GetGameMode)))
      (if (not (Class|DefaultGameMode|IsGameplayRunning _asbp_game_mode))
        (bind _aswb_main_menu (Utilities|Casting|CastToWB_MainMenu (UserInterface|GetUserWidgetObject (Variables|Default|GetMainMenuWidget))))
        (Default|Next _aswb_main_menu)))))

(event Input|ActionEvents|InputActionMenuUp
  (params (Key :type Key%20Structure :default "AnyKey"))
  ;[1 1 1] Prev Element
  (:Pressed
    (if (Rendering|IsVisible (Variables|Default|GetMainMenuWidget))
      (bind _asbp_game_mode (Utilities|Casting|CastToBP_GameMode (Game|GetGameMode)))
      (if (not (Class|DefaultGameMode|IsGameplayRunning _asbp_game_mode))
        (bind _aswb_main_menu (Utilities|Casting|CastToWB_MainMenu (UserInterface|GetUserWidgetObject (Variables|Default|GetMainMenuWidget))))
        (Default|Prev _aswb_main_menu)))))

(event Input|ActionEvents|InputActionMenuBack
  (params (Key :type Key%20Structure :default "AnyKey"))
  ;[1 1 1] Back
  (:Pressed
    (if (Rendering|IsVisible (Variables|Default|GetControllsWidget))
      (Rendering|SetVisibility (Variables|Default|GetControllsWidget) false false)
      (Rendering|SetVisibility (Variables|Default|GetMainMenuWidget) true false))))

(event Input|ActionEvents|InputActionResetHMD
  (params (Key :type Key%20Structure :default "AnyKey"))
  ;[1 1 1] Reset HMD Pos/Rot
  (:Pressed
    (Class|HeadMountedDisplayFunctionLibrary|ResetOrientationandPosition 0.0 "OrientationAndPosition")))

(fn ConstructionScript)

(fn Enable
  (Input|EnableInput (Game|GetPlayerController 0)))

(fn Disable
  (Input|DisableInput (Game|GetPlayerController 0)))