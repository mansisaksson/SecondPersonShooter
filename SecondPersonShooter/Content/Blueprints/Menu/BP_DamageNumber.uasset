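; BP_DamageNumber is a floating damage number actor that rises, fades out and then destroys itself.
; The construction script stores the start location and sets the text to the negated DamageValue.
; A Timeline started on BeginPlay drives the upward movement and the text's alpha fade.
; Each Tick, the text yaws to face the player character's possessed enemy rather than the camera.
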(event EventBeginPlay
  (bind _startlocation (Variables|Default|GetStartlocation))
  (bind _timeline (Variables|Default|GetTimeline))
  (bind _textrender (Variables|Default|GetTextRender))
  (bind _textrendercolor (Variables|/Script/Engine.TextRenderComponent|GetTextRenderColor _textrender))
  (bind _position (Timeline|Timeline PlayFromStart)
    (:Update
      (Transformation|SetActorLocation (Math|Vector|MakeVector (.x _startlocation) (.y _startlocation) (+ (.z _startlocation) (* _position 5e+01))) false false)
      (Rendering|Components|TextRender|SetTextRenderColor _textrender (Math|Color|MakeColor (.b _textrendercolor) (.g _textrendercolor) (.r _textrendercolor) (Math|Conversions|ToByte(Integer) (Math|Float|Truncate (* 255 (- 1.0 (/ (Components|Timeline|GetPlaybackPosition _timeline) (Components|Timeline|GetTimelineLength _timeline)))))))))
    (:Finished
      (Actor|DestroyActor))))

(event Collision|EventActorBeginOverlap
  (params (OtherActor :type Actor%20Object%20Reference)))

(event EventTick
  (params (DeltaSeconds :type Float%20%28single-precision%29))
  (bind _asbp_player_character (Utilities|Casting|CastToBP_PlayerCharacter (Game|Player|GetPlayerPawn 0)))
  (Transformation|SetWorldRotation (Variables|Default|GetTextRender) (Math|Rotator|MakeRotator 0.0 0.0 (.yaw (Math|Rotator|FindLookatRotation (Transformation|GetActorLocation) (Transformation|GetActorLocation (Class|PlayerCharacter|GetPossessedEnemy _asbp_player_character))))) false false))

(fn ConstructionScript
  (Rendering|Components|TextRender|SetText (Variables|Default|GetTextRender) (Utilities|Text|ToText(Float) (* (Variables|Default|GetDamageValue) -1.0) "HalfToEven"))
  (Variables|Default|SetStartlocation (Transformation|GetActorLocation)))