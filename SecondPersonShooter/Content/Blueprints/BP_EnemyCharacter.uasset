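; Enemy character with a wheel and lance that falls apart under physics on death and later despawns.
; While alive, Tick spins the wheel when moving; on death, it re-parents wheel and lance to the capsule and simulates their physics once.
; A dead-time counter destroys the actor after TimeToPhysics.
; Tick also positions and rotates a HUD widget from headset orientation and position.
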(event EventBeginPlay)

(event EventActorBeginOverlap
  (params (OtherActor :type Actor%20Object%20Reference)))

(event EventTick
  (params (DeltaSeconds :type Float%20%28single-precision%29))
  (bind (_devicerotation _deviceposition) (Class|HeadMountedDisplayFunctionLibrary|GetOrientationandPosition))
  (bind _widget (Variables|Default|GetWidget))
  (bind _returnvalue (+ (.yaw _devicerotation) 1.8e+02))
  (bind _returnvalue_2 (* (.pitch _devicerotation) -1.0))
  (bind _returnvalue_3 (* (.roll _devicerotation) -1.0))
  (Utilities|FlowControl|Sequence
    (:then_0
      ;[0.1408 1 0] HUD
      (Transformation|SetRelativeRotation _widget (Math|Rotator|MakeRotator _returnvalue_3 _returnvalue_2 _returnvalue) false false)
      (Transformation|SetRelativeLocation _widget (+ (* (Math|Rotator|GetRotationXVector (Math|Rotator|MakeRotator _returnvalue_3 _returnvalue_2 _returnvalue)) -11.0) _deviceposition) false false))
    (:then_1
      (if (Class|EnemyCharacter|GetIsAlive)
        ;[1 0 0.588] Wheel Rotation
        (Transformation|AddRelativeRotation (Variables|Default|GetWheel) (Math|Rotator|MakeRotator (* 5.0 (Math|Float|Clamp(Float) (Math|Vector|VectorLength (Variables|/Script/Engine.MovementComponent|GetVelocity (Pawn|GetMovementComponent))))) 0.0 0.0) false false)
        (Variables|Default|SetShouldWheelPhysics true)
        (else
          (Utilities|FlowControl|Sequence
            (:then_0
              ;[1 0.647 0] Enable Wheel/Lance Physics
              (if (Variables|Default|GetShouldWheelPhysics)
                (Class|SceneComponent|Attachto (Variables|Default|GetWheel) (Variables|Default|GetCapsuleComponent) "None" "KeepWorldPosition" true)
                (Physics|SetSimulatePhysics (Variables|Default|GetWheel) true)
                (Class|SceneComponent|Attachto (Variables|Default|GetLance) (Variables|Default|GetCapsuleComponent) "None" "KeepWorldPosition" true)
                (Collision|SetCollisionEnabled (Variables|Default|GetLance) "QueryAndPhysics")
                (Physics|SetSimulatePhysics (Variables|Default|GetLance) true)
                (Variables|Default|SetShouldWheelPhysics false)))
            (:then_1
              (Variables|Default|SetTimeSinceDead (+ (Variables|Default|GetTimeSinceDead) (Utilities|Time|GetWorldDeltaSeconds)))
              (Utilities|FlowControl|Sequence
                (:then_0
                  ;[0.5 0.2158 0] Disable physics
                  (if (> (Variables|Default|GetTimeSinceDead) (Variables|Default|GetTimeToPhysics))
                    (Physics|SetSimulatePhysics (Variables|Character|GetMesh) true)
                    (Physics|SetSimulatePhysics (Variables|Default|GetWheel) true)
                    (Physics|SetSimulatePhysics (Variables|Default|GetLance) true)))
                (:then_1
                  ;[1 0 0] Despawn
                  (if (> (Variables|Default|GetTimeSinceDead) (Variables|Default|GetTimeToPhysics))
                    (Actor|DestroyActor)))))))))))

(fn ConstructionScript)