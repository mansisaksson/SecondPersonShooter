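; BP_Enemy1 is a possessable robot enemy with a wheel and sword that appears as a red minimap dot.
; Player overlap with AttackArea triggers timed sword attacks that briefly open SwordCollider to deal damage, while Tick spins the wheel and toggles Head and ScreenSpace visibility during possession.
; Damage spawns floating numbers.
; Death detaches parts into physics, shows score and despawns after a delay, with SelfDestruct arming an explosion.
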(event OnComponentBeginOverlap(SwordCollider)
  (params (OverlappedComponent :type Primitive%20Component%20Object%20Reference) (OtherActor :type Actor%20Object%20Reference) (OtherComp :type Primitive%20Component%20Object%20Reference) (OtherBodyIndex :type Integer) (bFromSweep :type Boolean) (SweepResult :type Hit%20Result%20Structure%20%28by%20ref%29))
  (bind _asbp_player_character (Utilities|Casting|CastToBP_PlayerCharacter OtherActor))
  (Game|Damage|ApplyDamage _asbp_player_character 4e+01 0 self "/Script/Engine.DamageType"))

(event OnComponentBeginOverlap(AttackArea)
  (params (OverlappedComponent :type Primitive%20Component%20Object%20Reference) (OtherActor :type Actor%20Object%20Reference) (OtherComp :type Primitive%20Component%20Object%20Reference) (OtherBodyIndex :type Integer) (bFromSweep :type Boolean) (SweepResult :type Hit%20Result%20Structure%20%28by%20ref%29))
  (Utilities|Casting|CastToBP_PlayerCharacter OtherActor)
  (Variables|Default|SetIsInRange true))

(event OnComponentEndOverlap(AttackArea)
  (params (OverlappedComponent :type Primitive%20Component%20Object%20Reference) (OtherActor :type Actor%20Object%20Reference) (OtherComp :type Primitive%20Component%20Object%20Reference) (OtherBodyIndex :type Integer))
  (Utilities|Casting|CastToBP_PlayerCharacter OtherActor)
  (Variables|Default|SetIsInRange false))

(event Custom|OnTakeAnyDamage_Event_0
  (params (DamagedActor :type Actor%20Object%20Reference) (Damage :type Float%20%28single-precision%29) (DamageType :type Damage%20Type%20Object%20Reference) (InstigatedBy :type Controller%20Object%20Reference) (DamageCauser :type Actor%20Object%20Reference))
  (bind _returnvalue (Transformation|GetActorLocation))
  (Game|SpawnActorfromClass "/Game/Blueprints/Menu/BP_DamageNumber.BP_DamageNumber_C" (Math|Transform|MakeTransform (Math|Vector|MakeVector (.x _returnvalue) (.y _returnvalue) (+ (.z _returnvalue) 2e+01)) "0, 0, 0" "1,1,1") "AlwaysSpawn" 0 (Math|Float|Truncate Damage) 0))

(event EventOnDeath
  ;[0.535 0 0] On Enemy Death
  (Utilities|FlowControl|Sequence
    (:then_0
      ;;[1 1 1] Enable/Disable Component Physics
      (Collision|SetCollisionResponsetoAllChannels (Variables|Default|GetAttackArea) "ECR_Ignore")
      (Class|SceneComponent|DetachfromParent (Variables|Default|GetWheel) true true)
      (Physics|SetSimulatePhysics (Variables|Default|GetWheel) true)
      ;;[1 1 1] Remove from minimap
      (bind _asbp_game_mode (Utilities|Casting|CastToBP_GameMode (Game|GetGameMode)))
      (Utilities|IsValid (Variables|/Game/Blueprints/BP_GameMode.BP_GameMode_C|GetBP_MiniMap _asbp_game_mode)
        (:Is%20Valid
          (Default|RemoveActorfromMiniMap (Variables|/Game/Blueprints/BP_GameMode.BP_GameMode_C|GetBP_MiniMap _asbp_game_mode) self))))
    (:then_1
      ;;[1 1 1] Explode On Death
      (if (Variables|Default|GetExplodeOnDeath)
        (bind _returnvalue (Game|SpawnActorfromClass "/Game/Blueprints/BP_Explosion.BP_Explosion_C" (Math|Transform|MakeTransform (Transformation|GetActorLocation) "0, 0, 0" "1,1,1") "AlwaysSpawn" 0 0))
        (Default|Explode _returnvalue 1e+02 5.0 false)
        (bind _asbp_player_character (Utilities|Casting|CastToBP_PlayerCharacter (Game|GetPlayerCharacter 0)))
        (if (and (Class|PlayerCharacter|GetIsAlive _asbp_player_character) (== (Class|PlayerCharacter|GetPossessedEnemy _asbp_player_character) self))
          (Class|PlayerCharacter|PossessedIsKilled _asbp_player_character))))
    (:then_2
      ;;[1 1 1] ShowScore
      (bind _asplayer_character (Utilities|Casting|CastToPlayerCharacter (Game|Player|GetPlayerPawn 0)))
      (Game|SpawnActorfromClass "/Game/Blueprints/Menu/BP_ScoreNumber.BP_ScoreNumber_C" (Math|Transform|MakeTransform (Math|Vector|MakeVector (.x (Transformation|GetActorLocation _asplayer_character)) (.y (Transformation|GetActorLocation _asplayer_character)) (+ (.z (Transformation|GetActorLocation _asplayer_character)) 2e+01)) "0, 0, 0" "1,1,1") "Undefined" 0 (Variables|Default|GetscoreGivenOnDeath) 0))
    (:then_3
      ;;[1 1 1] Despawn Dead Enemy
      (Utilities|FlowControl|Delay (Variables|Default|GetTimeToDespawn))
      (Actor|DestroyActor))))

(event EventBeginPlay
  (Utilities|FlowControl|Sequence
    (:then_0
      (bind _asbp_game_mode (Utilities|Casting|CastToBP_GameMode (Game|GetGameMode)))
      (Utilities|IsValid (Variables|/Game/Blueprints/BP_GameMode.BP_GameMode_C|GetBP_MiniMap _asbp_game_mode)
        (:Is%20Valid
          (Default|AddActortoMiniMap (Variables|/Game/Blueprints/BP_GameMode.BP_GameMode_C|GetBP_MiniMap _asbp_game_mode) self "/Game/Assets/Textures/MiniMap/SPR_MapDott_Red.SPR_MapDott_Red"))
        (:Is%20Not%20Valid
          (bind _outactors (Actor|GetAllActorsOfClass "/Game/Blueprints/BP_MiniMap.BP_MiniMap_C"))
          (for _array_element _outactors
            (Default|AddActortoMiniMap _array_element self "/Game/Assets/Textures/MiniMap/SPR_MapDott_Red.SPR_MapDott_Red")))))
    (:then_1
      (EventDispatchers|BindEventtoOnTakeAnyDamage (delegate Custom|OnTakeAnyDamage_Event_0)))))

(event EventTick
  (params (DeltaSeconds :type Float%20%28single-precision%29))
  (bind _asbp_game_mode (Utilities|Casting|CastToBP_GameMode (Game|GetGameMode)))
  (if (Class|DefaultGameMode|IsGameplayRunning _asbp_game_mode)
    (Utilities|FlowControl|Sequence
      (:then_0
        ;[1 1 1] Hide/Show HUD
        (bind _asbp_player_character (Utilities|Casting|CastToBP_PlayerCharacter (Game|Player|GetPlayerPawn 0) :!label _label))
        (Development|SetHiddeninGame (Variables|Default|GetScreenSpace) (not (== (Class|PlayerCharacter|GetPossessedEnemy _asbp_player_character) self)) false)
        (Development|SetHiddeninGame (Variables|Default|GetHead) (== (Class|PlayerCharacter|GetPossessedEnemy _asbp_player_character) self) false))
      (:then_1
        (if (Class|EnemyCharacter|GetIsAlive)
          (Utilities|FlowControl|Sequence
            (:then_0
              ;[1 0 0.588] Wheel Rotation
              (if (Variables|Default|GetSpinWheel)
                (Transformation|AddRelativeRotation (Variables|Default|GetWheel) (Math|Rotator|MakeRotator (* 5.0 (Math|Float|Clamp(Float) (Math|Vector|VectorLength (Variables|/Script/Engine.MovementComponent|GetVelocity (Pawn|GetMovementComponent))))) 0.0 0.0) false false)))
            (:then_1
              ;[0.4093 1 0] Attack Player
              (if (Variables|Default|GetIsInRange)
                (if (Variables|Default|GetCanAttack)
                  (Variables|Default|SetCanAttack false)
                  (Collision|SetCollisionResponsetoAllChannels (Variables|Default|GetSwordCollider) "ECR_Overlap")
                  (CallFunction|PlayAttackAnim)
                  (Utilities|FlowControl|Sequence
                    (:then_0
                      (Utilities|FlowControl|Delay 2.0)
                      (Variables|Default|SetCanAttack true))
                    (:then_1
                      (Utilities|FlowControl|Delay 0.8)
                      (Collision|SetCollisionResponsetoAllChannels (Variables|Default|GetSwordCollider) "ECR_Ignore"))))))))))
    (else
      (goto _label))))

(fn ConstructionScript
  (Class|SceneComponent|Attachto (Variables|Default|GetExhaust1) (Variables|Character|GetMesh) "Exhaust" "KeepRelativeOffset" true)
  (Class|SceneComponent|Attachto (Variables|Default|GetSword) (Variables|Character|GetMesh) "Sword" "KeepRelativeOffset" true))

(fn SelfDestruct
  (Class|EnemyCharacter|DisableEnemy 1.45 true true)
  (Variables|Default|SetExplodeOnDeath true)
  (Audio|PlaySoundatLocation "/Game/Assets/Audio/countdownsound.countdownsound" (Transformation|GetActorLocation)))

(fn PlayAttackAnim
  (bind _asabp_robot_3_no_shield (Utilities|Casting|CastToABP_Robot3_NoShield (Components|SkeletalMesh|GetAnimInstance (Variables|Character|GetMesh))))
  (Default|PlayAttackAnim _asabp_robot_3_no_shield))