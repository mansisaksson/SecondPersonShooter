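; BP_SpeedPickup is a collectible that permanently raises the player's movement speed when touched.
; On overlap with BP_PlayerCharacter it adds an amount inversely proportional to the current MaxWalkSpeed, giving diminishing returns, then plays a sound and destroys itself.
; Tick animates it with a sine-driven vertical bob, applied per frame without delta-time scaling, and a slow delta-time-scaled yaw spin.
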(event EventBeginPlay)

(event EventActorBeginOverlap
  (params (OtherActor :type Actor%20Object%20Reference))
  (bind _asbp_player_character (Utilities|Casting|CastToBP_PlayerCharacter OtherActor))
  (Variables|/Script/Engine.CharacterMovementComponent|SetMaxWalkSpeed (Variables|/Script/Engine.Character|GetCharacterMovement _asbp_player_character) (+ (Variables|/Script/Engine.CharacterMovementComponent|GetMaxWalkSpeed (Variables|/Script/Engine.Character|GetCharacterMovement _asbp_player_character)) (/ 1e+04 (Variables|/Script/Engine.CharacterMovementComponent|GetMaxWalkSpeed (Variables|/Script/Engine.Character|GetCharacterMovement _asbp_player_character)))))
  (Audio|PlaySoundatLocation "/Game/Assets/Audio/speed.speed" (Transformation|GetActorLocation))
  (Actor|DestroyActor))

(event EventTick
  (params (DeltaSeconds :type Float%20%28single-precision%29))
  (bind _returnvalue (Transformation|GetActorLocation))
  (bind _returnvalue_2 (Transformation|GetActorRotation))
  (Transformation|SetActorLocation (Math|Vector|MakeVector (.x _returnvalue) (.y _returnvalue) (+ (.z _returnvalue) (* (Math|Trig|Sin(Radians) (* (Utilities|Time|GetGameTimeinSeconds) 1.0)) 0.2))) false false)
  (Transformation|SetActorRotation (Math|Rotator|MakeRotator (.roll _returnvalue_2) (.pitch _returnvalue_2) (+ (.yaw _returnvalue_2) (* (Utilities|Time|GetWorldDeltaSeconds) 6.0)))))

(fn ConstructionScript)