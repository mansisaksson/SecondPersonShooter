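; BP_Pickup_HP is a health pickup that restores a fixed amount of the player's health, capped at maximum.
; Tick bobs it on a sine wave, applied as a per-frame offset, and spins it on all axes.
; Overlap events track the player, and Tick polls that state, so pickup waits until health is below max.
; Collection calls OnStatusChanged before raising health, plays the Ammopickup sound, removes the minimap entry and destroys the actor.
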(event Collision|EventActorEndOverlap
  (params (OtherActor :type Actor%20Object%20Reference))
  (bind _asbp_player_character (Utilities|Casting|CastToBP_PlayerCharacter OtherActor))
  (Variables|Default|SetOverlappingPlayer false)
  (Variables|Default|SetPlayerRef _asbp_player_character))

(event EventBeginPlay)

(event Collision|EventActorBeginOverlap
  (params (OtherActor :type Actor%20Object%20Reference))
  (bind _asbp_player_character (Utilities|Casting|CastToBP_PlayerCharacter OtherActor))
  (Variables|Default|SetOverlappingPlayer true)
  (Variables|Default|SetPlayerRef _asbp_player_character))

(event EventTick
  (params (DeltaSeconds :type Float%20%28single-precision%29))
  (bind _returnvalue (Utilities|Time|GetWorldDeltaSeconds))
  (bind _playerref (Variables|Default|GetPlayerRef))
  (bind _returnvalue_2 (Class|PlayerCharacter|GetMaxHealth _playerref))
  (bind _returnvalue_3 (* _returnvalue 6e+01))
  (Utilities|FlowControl|Sequence
    (:then_0
      (Transformation|AddWorldOffset (Variables|Default|GetDefaultSceneRoot) (Math|Vector|MakeVector 0.0 0.0 (* (Math|Trig|Sin(Radians) (* (Utilities|Time|GetGameTimeinSeconds) 2.0)) 0.2)) false false)
      (Transformation|AddLocalRotation (Variables|Default|GetDefaultSceneRoot) (Math|Rotator|MakeRotator _returnvalue_3 _returnvalue_3 _returnvalue_3) false false))
    (:then_1
      (if (Variables|Default|GetOverlappingPlayer)
        (if (< (Variables|/Script/SecondPersonShooter.PlayerCharacter|GetHealth _playerref) _returnvalue_2)
          (Default|OnStatusChanged _playerref)
          (Variables|/Script/SecondPersonShooter.PlayerCharacter|SetHealth _playerref (Math|Float|Clamp(Float) (+ (Variables|/Script/SecondPersonShooter.PlayerCharacter|GetHealth _playerref) 3e+01) 0.0 _returnvalue_2))
          (Audio|PlaySoundatLocation "/Game/Assets/Audio/ammo-pick-up.ammo-pick-up" (Transformation|GetActorLocation))
          (Default|RemoveActorfromMiniMap (Variables|Default|GetMinimap) self)
          (Actor|DestroyActor))))))

(fn ConstructionScript)