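; VR player character with HMD tracking and orientation reset, laser sight, toggleable stats display and an energy-costing EMP special.
; Tick traces to place the laser beam's endpoint and turns the stats display toward the possessed enemy.
; After death, a delay triggers a one-time blend to the death camera and clears the possessed enemy.
; OnFire plays the animation through ABP_SuperGuy, and construction attaches backpack and head meshes to sockets.
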(event EventBeginPlay
  ;[1 1 1] Enable Head Mounted Display
  (Class|HeadMountedDisplayFunctionLibrary|EnableHMD true)
  (Variables|/Script/Engine.PlayerCameraManager|SetbFollowHmdOrientation (Game|GetPlayerCameraManager 0) true)
  (Rendering|SetVisibility (Variables|Default|GetPlayerStats) false false)
  (Variables|Default|SetSpecialWeapon "NewEnumerator0"))

(event EventTick
  (params (DeltaSeconds :type Float%20%28single-precision%29))
  (bind _returnvalue (Class|PlayerCharacter|GetPossessedEnemy))
  (Utilities|FlowControl|Sequence
    (:then_0
      ;[1 0 0.01801] Fixa Laser Siktet
      (bind (_outhit _returnvalue_2) (Collision|LineTraceForObjects (Transformation|GetWorldLocation (Variables|Default|GetBulletSpawnComp)) (* (Math|Rotator|GetRotationXVector (Transformation|GetWorldRotation (Variables|Default|GetCapsuleComponent))) 5e+04) (Utilities|Array|MakeArray "ObjectTypeQuery1" "ObjectTypeQuery4" "ObjectTypeQuery2") false 0 "None"))
      (if _returnvalue_2
        (Class|ParticleSystemComponent|SetBeamEndPoint (Variables|Default|GetLaser%20Sight) 0 (.Location (Collision|BreakHitResult _outhit)))))
    (:then_1
      ;[0.05324 1 0] Update Player HUD
      (Utilities|IsValid _returnvalue
        (:Is%20Valid
          (Transformation|SetWorldRotation (Variables|Default|GetPlayerStats) (Math|Rotator|MakeRotfromX (- (Transformation|GetActorLocation _returnvalue) (Transformation|GetActorLocation))) false false))))
    (:then_2
      ;[1 0.3464 0.1438] Scoreboard när man dör
      (if (not (Class|PlayerCharacter|GetIsAlive))
        (Variables|Default|SetTimeSinceDeath (+ (Variables|Default|GetTimeSinceDeath) (Utilities|Time|GetWorldDeltaSeconds)))
        (if (> (Variables|Default|GetTimeSinceDeath) (Variables|Default|GetTime%20To%20swich%20Camera))
          (Utilities|FlowControl|DoOnce false
            (:Completed
              (bind _asplayer_controller (Utilities|Casting|CastToPlayerController (Pawn|GetController)))
              (bind _outactors (Actor|GetAllActorsOfClass "/Game/Blueprints/BP_DeathCamera.BP_DeathCamera_C"))
              (for _array_element _outactors
                (Game|Player|SetViewTargetwithBlend _asplayer_controller _array_element 5.0 "VTBlend_Linear" 0.0 false)
                (Class|PlayerCharacter|ClearPossessedEnemy)))))))))

(event EventOnFire
  ;[1 1 1] Player Fire Anim
  (bind _asabp_super_guy (Utilities|Casting|CastToABP_SuperGuy (Components|SkeletalMesh|GetAnimInstance (Variables|Character|GetMesh))))
  (Default|PlayFireAnim _asabp_super_guy))

(event Input|ActionEvents|InputActionFireSpecial
  (params (Key :type Key%20Structure :default "AnyKey"))
  (:Pressed
    (switch Utilities|FlowControl|Switch|SwitchonEN_SpecialWeapons (Variables|Default|GetSpecialWeapon)
      (:NewEnumerator0
        (if (>= (Class|PlayerCharacter|GetSpecial) 2e+01)
          (Game|SpawnActorfromClass "/Game/Blueprints/BP_EMP.BP_EMP_C" (Math|Transform|MakeTransform (Transformation|GetActorLocation) "0, 0, 0" "1,1,1") "AlwaysSpawn" 0 0)
          (Variables|Default|SetSpecial (- (Class|PlayerCharacter|GetSpecial) 2e+01)))))))

(event Input|ActionEvents|InputActionResetHMD
  (params (Key :type Key%20Structure :default "AnyKey"))
  ;[1 1 1] Reset HMD Pos/Rot
  (:Pressed
    (Class|HeadMountedDisplayFunctionLibrary|ResetOrientationandPosition 0.0 "OrientationAndPosition")))

(event Input|ActionEvents|InputActionDisplayPlayerStats
  (params (Key :type Key%20Structure :default "AnyKey"))
  (bind _playerstats (Variables|Default|GetPlayerStats))
  ;[1 1 1] Show/Hide Player HUD
  (:Pressed
    (Rendering|SetVisibility _playerstats true false))
  (:Released
    (Rendering|SetVisibility _playerstats false false)))

(fn ConstructionScript
  (Class|SceneComponent|Attachto (Variables|Default|GetBackPack) (Variables|Character|GetMesh) "BackPack" "KeepWorldPosition" true)
  (Class|SceneComponent|Attachto (Variables|Default|GetStaticMesh) (Variables|Character|GetMesh) "Head" "KeepRelativeOffset" true))