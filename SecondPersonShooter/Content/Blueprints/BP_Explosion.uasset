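; BP_Explosion is a short-lived explosion actor that deals damage through an overlap sphere and removes itself about one frame after it starts ticking.
; Explode stores damage and friendly-fire settings, enables sphere overlaps and spawns a particle effect at the given scale.
; Each overlapped actor takes damage once, with players exempt unless FriendlyFire is set.
; Physics-simulating components also receive an impulse directed toward the explosion's center.
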(event OnComponentBeginOverlap(Sphere)
  (params (OtherActor :type Actor%20Object%20Reference) (OtherComp :type Primitive%20Component%20Object%20Reference) (OtherBodyIndex :type Integer) (bFromSweep :type Boolean) (SweepResult :type Hit%20Result%20Structure%20%28by%20ref%29))
  (Utilities|Casting|CastToBP_PlayerCharacter OtherActor
    (:then
      (if (Variables|Default|GetFriendlyFire)
        (if (not (Utilities|Array|ContainsItem (Variables|Default|GetHitActors) OtherActor)) :!label _label
          (Utilities|Array|Add (Variables|Default|GetHitActors) OtherActor)
          (Game|Damage|ApplyDamage OtherActor (Variables|Default|GetDamage) 0 self "/Script/Engine.DamageType")
          (if (Physics|IsSimulatingPhysics OtherComp "None")
            (Physics|AddImpulse OtherComp (* (Math|Vector|Normalize (- (Transformation|GetActorLocation) (Transformation|GetWorldLocation OtherComp))) 1e+04) "None" false)))))
    (:CastFailed
      (goto _label))))

(event EventTick
  (params (DeltaSeconds :type Float%20%28single-precision%29))
  (Utilities|FlowControl|Delay (Utilities|Time|GetWorldDeltaSeconds))
  (Actor|DestroyActor))

(fn ConstructionScript)

(fn Explode
  (params (Damage :type Float%20%28single-precision%29) (Scale :type Float%20%28single-precision%29) (FriendlyFire :type Boolean))
  (bind _sphere (Variables|Default|GetSphere))
  (Variables|Default|SetFriendlyFire FriendlyFire)
  (Variables|Default|SetDamage Damage)
  (Collision|SetCollisionEnabled _sphere "QueryAndPhysics")
  (Collision|SetCollisionResponsetoAllChannels _sphere "ECR_Overlap")
  (bind _returnvalue (Effects|SpawnEmitteratLocation "/Game/PluginContent/StarterContent/Particles/P_Explosion.P_Explosion" (Transformation|GetActorLocation)))
  (Transformation|SetWorldScale3D _returnvalue (* (Math|Vector|MakeVector 1.0 1.0 1.0) Scale)))