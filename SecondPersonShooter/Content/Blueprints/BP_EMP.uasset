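; BP_EMP is a short-lived EMP blast actor that temporarily disables enemies it overlaps.
; On BeginPlay it sets its Sphere to overlap all channels, enables collision and spawns an explosion particle at its location.
; Sphere overlaps cast to BP_EnemyCharacter and call DisableEnemy without blocking damage or killing on finish.
; A Delay on Tick destroys the actor a fraction of a second after it spawns.
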(event OnComponentBeginOverlap(Sphere)
  (params (OtherActor :type Actor%20Object%20Reference) (OtherComp :type Primitive%20Component%20Object%20Reference) (OtherBodyIndex :type Integer) (bFromSweep :type Boolean) (SweepResult :type Hit%20Result%20Structure%20%28by%20ref%29))
  (bind _asbp_enemy_character (Utilities|Casting|CastToBP_EnemyCharacter OtherActor))
  (Class|EnemyCharacter|DisableEnemy _asbp_enemy_character 2.0 false false))

(event EventBeginPlay
  (bind _sphere (Variables|Default|GetSphere))
  (Collision|SetCollisionResponsetoAllChannels _sphere "ECR_Overlap")
  (Collision|SetCollisionEnabled _sphere "QueryAndPhysics")
  (Effects|SpawnEmitteratLocation "/Game/PluginContent/StarterContent/Particles/P_Explosion.P_Explosion" (Transformation|GetActorLocation)))

(event EventActorBeginOverlap
  (params (OtherActor :type Actor%20Object%20Reference)))

(event EventTick
  (params (DeltaSeconds :type Float%20%28single-precision%29))
  (Utilities|FlowControl|Delay 0.1)
  (Actor|DestroyActor))

(fn ConstructionScript)