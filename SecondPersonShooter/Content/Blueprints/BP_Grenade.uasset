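; Grenade actor that explodes after a fuse delay or on hitting an EnemyCharacter, spawning an explosion particle at its location.
; Explode enables overlap on a CollisionSphere as the blast area, and enemies entering that overlap take damage.
; Once HasExploded is set, Tick destroys the actor after a short delay, leaving a brief window for the overlap damage to register.
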(event OnComponentHit(Sphere)
  (params (OtherActor :type Actor%20Object%20Reference) (OtherComp :type Primitive%20Component%20Object%20Reference) (NormalImpulse :type Vector :default "0, 0, 0") (Hit :type Hit%20Result%20Structure%20%28by%20ref%29))
  (Utilities|Casting|CastToEnemyCharacter OtherActor)
  (Effects|SpawnEmitteratLocation "/Game/PluginContent/StarterContent/Particles/P_Explosion.P_Explosion" (Transformation|GetActorLocation))
  (CallFunction|Explode))

(event OnComponentBeginOverlap(CollisionSphere)
  (params (OtherActor :type Actor%20Object%20Reference) (OtherComp :type Primitive%20Component%20Object%20Reference) (OtherBodyIndex :type Integer) (bFromSweep :type Boolean) (SweepResult :type Hit%20Result%20Structure%20%28by%20ref%29))
  (bind _asenemy_character (Utilities|Casting|CastToEnemyCharacter OtherActor))
  (Game|Damage|ApplyDamage _asenemy_character 1e+02 0 self "/Script/Engine.DamageType"))

(event EventBeginPlay
  (Utilities|FlowControl|Delay 3.0)
  (Effects|SpawnEmitteratLocation "/Game/PluginContent/StarterContent/Particles/P_Explosion.P_Explosion" (Transformation|GetActorLocation))
  (CallFunction|Explode))

(event Collision|EventActorBeginOverlap
  (params (OtherActor :type Actor%20Object%20Reference)))

(event EventTick
  (params (DeltaSeconds :type Float%20%28single-precision%29))
  (if (Variables|Default|GetHasExploded)
    (Utilities|FlowControl|Delay 0.2)
    (Actor|DestroyActor)))

(fn ConstructionScript)

(fn Explode
  (bind _collisionsphere (Variables|Default|GetCollisionSphere))
  (Collision|SetCollisionEnabled _collisionsphere "QueryAndPhysics")
  (Collision|SetCollisionResponsetoAllChannels _collisionsphere "ECR_Overlap")
  (Variables|Default|SetHasExploded true))