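; BP_PickupSpeed is a speed pickup that permanently raises the walk speed of a BP_PlayerCharacter that overlaps it.
; On overlap it adds a bonus inversely proportional to the current MaxWalkSpeed, giving diminishing returns on repeated pickups, then plays a sound and destroys itself.
; Tick bobs the root with a sine-driven world offset, which is not scaled by delta time, and spins it on all three axes.
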(event EventBeginPlay)

(event EventActorBeginOverlap
  (params (OtherActor :type Actor%20Object%20Reference))
  (bind _asbp_player_character (Utilities|Casting|CastToBP_PlayerCharacter OtherActor))
  (Variables|/Script/Engine.CharacterMovementComponent|SetMaxWalkSpeed (Variables|/Script/Engine.Character|GetCharacterMovement _asbp_player_character) (+ (Variables|/Script/Engine.CharacterMovementComponent|GetMaxWalkSpeed (Variables|/Script/Engine.Character|GetCharacterMovement _asbp_player_character)) (/ 1e+04 (Variables|/Script/Engine.CharacterMovementComponent|GetMaxWalkSpeed (Variables|/Script/Engine.Character|GetCharacterMovement _asbp_player_character)))))
  (Audio|PlaySoundatLocation "/Game/Assets/Audio/speed.speed" (Transformation|GetActorLocation))
  (Actor|DestroyActor))

(event EventTick
  (params (DeltaSeconds :type Float%20%28single-precision%29))
  (bind _returnvalue (Utilities|Time|GetWorldDeltaSeconds))
  (bind _returnvalue_2 (* _returnvalue 6e+01))
  (Transformation|AddWorldOffset (Variables|Default|GetDefaultSceneRoot) (Math|Vector|MakeVector 0.0 0.0 (* (Math|Trig|Sin(Radians) (* (Utilities|Time|GetGameTimeinSeconds) 2.0)) 0.2)) false false)
  (Transformation|AddLocalRotation (Variables|Default|GetDefaultSceneRoot) (Math|Rotator|MakeRotator _returnvalue_2 _returnvalue_2 _returnvalue_2) false false))

(fn ConstructionScript)