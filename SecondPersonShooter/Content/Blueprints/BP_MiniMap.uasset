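; Minimap actor that shows registered actors as Paper2D sprites, centered on the enemy the player currently possesses.
; Add and remove events maintain parallel actor and sprite lists, and Tick maps scaled world positions and yaw onto the sprites.
; Offsetting the sprite parent and counter-rotating the scene keeps the possessed enemy centered.
; When possession changes, the map reattaches to that enemy's MiniMap socket and swaps red and white dots.
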(event Custom|AddActorToMiniMap
  (params (Actor :type Actor%20Object%20Reference) (Sprite :type Paper%20Sprite%20Object%20Reference))
  (bind _currentparent (Variables|Default|GetCurrentParent))
  (bind _actorlist (Variables|MiniMap|GetActorList))
  (bind _spritelist (Variables|MiniMap|GetSpriteList))
  (bind _returnvalue (Utilities|Array|FindItem _actorlist _currentparent))
  (bind _item (Utilities|Array|Get(acopy) _spritelist _returnvalue))
  ;[0.1258 0.775 0.1201] Add Actor To MiniMap
  (bind _returnvalue_2 (Utilities|Array|AddUnique (Variables|MiniMap|GetActorList) Actor))
  (if (!= _returnvalue_2 -1) ; Actor does not exist?
    (bind _returnvalue_3 (AddComponent|AddPaperSpriteComponent false))
    (Rendering|Components|Sprite|SetSprite _returnvalue_3 Sprite)
    (Utilities|Array|Add (Variables|MiniMap|GetSpriteList) _returnvalue_3)
    (Collision|SetCollisionEnabled _returnvalue_3 "NoCollision")
    (Class|SceneComponent|Attachto _returnvalue_3 (Variables|Default|GetSprParent) "None" "KeepRelativeOffset" true)
    ;[1 1 1] Update Positions and Angels
    (for (_array_element _array_index) (Variables|MiniMap|GetActorList)
      (Transformation|SetRelativeLocationAndRotation (Utilities|Array|Get(acopy) (Variables|MiniMap|GetSpriteList) _array_index) (Math|Vector|MakeVector (* (.X (Math|Vector|BreakVector (Transformation|GetActorLocation _array_element))) 0.025) 0.0 (* (.Y (Math|Vector|BreakVector (Transformation|GetActorLocation _array_element))) 0.025)) (Math|Rotator|MakeRotator 0.0 (.Yaw (Math|Rotator|BreakRotator (Transformation|GetActorRotation _array_element))) 0.0) false false))
    ;[1 1 1] Set map center to parent pos and rot
    (Utilities|IsValid _currentparent
      (:Is%20Valid
        (Utilities|IsValid _item
          (:Is%20Valid
            (Transformation|SetRelativeLocation (Variables|Default|GetSprParent) (* (Variables|/Script/Engine.SceneComponent|GetRelativeLocation _item) -1.0) false false)
            (Transformation|SetRelativeRotation (Variables|Default|GetScene) (Math|Rotator|CombineRotators (* (Variables|/Script/Engine.SceneComponent|GetRelativeRotation _item) -1.0) "90.000000, 0, 0") false false)))))))

(event Custom|RemoveActorFromMiniMap
  (params (Actor :type Actor%20Object%20Reference))
  (bind _spritelist (Variables|MiniMap|GetSpriteList))
  ;[1 0.159 0.1973] Remove Actor From MiniMap
  (bind _output_get (Variables|MiniMap|SetTempIndex (Utilities|Array|FindItem (Variables|MiniMap|GetActorList) Actor)))
  (if (!= _output_get -1) ; Actor exists in list?
    (Utilities|Array|RemoveIndex (Variables|MiniMap|GetActorList) _output_get)
    (Components|DestroyComponent (Utilities|Array|Get(acopy) _spritelist _output_get))
    (Utilities|Array|RemoveIndex _spritelist _output_get)))

(event EventTick
  (params (DeltaSeconds :type Float%20%28single-precision%29))
  (Utilities|FlowControl|Sequence
    (:then_0
      ;[1 1 1] Update Positions and Angels
      (for (_array_element _array_index) (Variables|MiniMap|GetActorList)
        (Transformation|SetRelativeLocationAndRotation (Utilities|Array|Get(acopy) (Variables|MiniMap|GetSpriteList) _array_index) (Math|Vector|MakeVector (* (.X (Math|Vector|BreakVector (Transformation|GetActorLocation _array_element))) 0.025) 0.0 (* (.Y (Math|Vector|BreakVector (Transformation|GetActorLocation _array_element))) 0.025)) (Math|Rotator|MakeRotator 0.0 (.Yaw (Math|Rotator|BreakRotator (Transformation|GetActorRotation _array_element))) 0.0) false false))
      ;[1 1 1] Set map center to parent pos and rot
      (Utilities|IsValid (Variables|Default|GetCurrentParent)
        (:Is%20Valid
          (Utilities|IsValid (Utilities|Array|Get(acopy) (Variables|MiniMap|GetSpriteList) (Utilities|Array|FindItem (Variables|MiniMap|GetActorList) (Variables|Default|GetCurrentParent)))
            (:Is%20Valid
              (Transformation|SetRelativeLocation (Variables|Default|GetSprParent) (* (Variables|/Script/Engine.SceneComponent|GetRelativeLocation (Utilities|Array|Get(acopy) (Variables|MiniMap|GetSpriteList) (Utilities|Array|FindItem (Variables|MiniMap|GetActorList) (Variables|Default|GetCurrentParent)))) -1.0) false false)
              (Transformation|SetRelativeRotation (Variables|Default|GetScene) (Math|Rotator|CombineRotators (* (Variables|/Script/Engine.SceneComponent|GetRelativeRotation (Utilities|Array|Get(acopy) (Variables|MiniMap|GetSpriteList) (Utilities|Array|FindItem (Variables|MiniMap|GetActorList) (Variables|Default|GetCurrentParent)))) -1.0) "90.000000, 0, 0") false false))))))
    (:then_1
      ;[1 1 1] Change parent
      (bind _asbp_player_character (Utilities|Casting|CastToBP_PlayerCharacter (Game|GetPlayerCharacter 0)))
      (if (and (Class|PlayerCharacter|GetIsAlive _asbp_player_character) (!= (Class|PlayerCharacter|GetPossessedEnemy _asbp_player_character) (Variables|Default|GetCurrentParent)))
        (Utilities|FlowControl|Sequence
          (:then_0
            ;[1 1 1] Set previous parent sprite to red
            (Utilities|IsValid (Variables|Default|GetCurrentParent)
              (:Is%20Valid
                (Utilities|IsValid (Utilities|Array|Get(acopy) (Variables|MiniMap|GetSpriteList) (Utilities|Array|FindItem (Variables|MiniMap|GetActorList) (Variables|Default|GetCurrentParent)))
                  (:Is%20Valid
                    (Rendering|Components|Sprite|SetSprite (Utilities|Array|Get(acopy) (Variables|MiniMap|GetSpriteList) (Utilities|Array|FindItem (Variables|MiniMap|GetActorList) (Variables|Default|GetCurrentParent))) "/Game/Assets/Textures/MiniMap/SPR_MapDott_Red.SPR_MapDott_Red"))))))
          (:then_1
            (Variables|Default|SetCurrentParent (Class|PlayerCharacter|GetPossessedEnemy _asbp_player_character))
            (Class|SceneComponent|Attachto (Variables|Default|GetDefaultSceneRoot) (Variables|/Script/Engine.Character|GetMesh (Class|PlayerCharacter|GetPossessedEnemy _asbp_player_character)) "MiniMap" "KeepRelativeOffset" true)
            (Transformation|SetActorRelativeLocation "0, 0, 0")
            ;[1 1 1] Set current parent sprite to white
            (Rendering|Components|Sprite|SetSprite (Utilities|Array|Get(acopy) (Variables|MiniMap|GetSpriteList) (Utilities|Array|FindItem (Variables|MiniMap|GetActorList) (Variables|Default|GetCurrentParent))) "/Game/Assets/Textures/MiniMap/SPR_MapDott_White.SPR_MapDott_White")))))))

(event EventBeginPlay
  (Transformation|SetWorldLocation (Variables|Default|GetDefaultSceneRoot) "0, 0, 0" false false))

(fn ConstructionScript)