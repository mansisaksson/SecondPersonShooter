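; Speed powerup pickup that boosts the movement and fire rate of the BP_PlayerCharacter that overlaps it.
; Overlap extends the super speed timer, sets an attack speed bonus, doubles walk speed, and raises base move speed and shots per second with diminishing returns.
; It attaches foot particles, plays a sound, then destroys itself.
; It shows a green minimap sprite and bobs and spins on Tick.
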(event EventBeginPlay
  (Variables|Default|SetMinimapSprite "/Game/Assets/Textures/MiniMap/SPR_MapPowerup_Green.SPR_MapPowerup_Green")
  (|CallParentFunction))

(event EventActorBeginOverlap
  (params (OtherActor :type Actor%20Object%20Reference))
  (bind _asbp_player_character (Utilities|Casting|CastToBP_PlayerCharacter OtherActor))
  (Effects|SpawnEmitterAttached "/Game/Assets/Particles/P_SpeedBonus.P_SpeedBonus" (Variables|/Script/Engine.Character|GetMesh _asbp_player_character) "LeftFoot" "0,0.000000,20.000000")
  (Effects|SpawnEmitterAttached "/Game/Assets/Particles/P_SpeedBonus.P_SpeedBonus" (Variables|/Script/Engine.Character|GetMesh _asbp_player_character) "RightFoot" "0,0.000000,20.000000")
  (Variables|/Script/SecondPersonShooter.PlayerCharacter|SetSuperSpeedTime _asbp_player_character (+ (Variables|/Script/SecondPersonShooter.PlayerCharacter|GetSuperSpeedTime _asbp_player_character) 5.0))
  (Variables|/Script/SecondPersonShooter.PlayerCharacter|SetShotsPerSecond _asbp_player_character (+ (Variables|/Script/SecondPersonShooter.PlayerCharacter|GetShotsPerSecond _asbp_player_character) (/ 2.0 (Variables|/Script/SecondPersonShooter.PlayerCharacter|GetShotsPerSecond _asbp_player_character))))
  (Variables|/Script/SecondPersonShooter.PlayerCharacter|SetAttackSpeedBonus _asbp_player_character 3.0)
  (bind _output_get (Variables|/Script/SecondPersonShooter.PlayerCharacter|SetDefaultMaxMoveSpeed _asbp_player_character (+ (Variables|/Script/SecondPersonShooter.PlayerCharacter|GetDefaultMaxMoveSpeed _asbp_player_character) (Math|Float|Sqrt (- 1e+03 (Variables|/Script/SecondPersonShooter.PlayerCharacter|GetDefaultMaxMoveSpeed _asbp_player_character))))))
  (Variables|/Script/Engine.CharacterMovementComponent|SetMaxWalkSpeed (Variables|/Script/Engine.Character|GetCharacterMovement _asbp_player_character) (* _output_get 2.0))
  (Audio|PlaySoundatLocation "/Game/Assets/Audio/speed.speed" (Transformation|GetActorLocation))
  (Actor|DestroyActor))

(event EventTick
  (params (DeltaSeconds :type Float%20%28single-precision%29))
  (bind _returnvalue (Utilities|Time|GetWorldDeltaSeconds))
  (bind _returnvalue_2 (* _returnvalue 6e+01))
  (Transformation|AddWorldOffset (Variables|Default|GetDefaultSceneRoot) (Math|Vector|MakeVector 0.0 0.0 (* (Math|Trig|Sin(Radians) (* (Utilities|Time|GetGameTimeinSeconds) 2.0)) 0.2)) false false)
  (Transformation|AddLocalRotation (Variables|Default|GetDefaultSceneRoot) (Math|Rotator|MakeRotator _returnvalue_2 _returnvalue_2 _returnvalue_2) false false))

(fn ConstructionScript)