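; BP_Pickup_Weapon is a pickup that grants the player a temporary Laser super weapon.
; On overlap with BP_PlayerCharacter it sets the weapon, super weapon duration and speed on the character, plays a pickup sound and destroys itself.
; BeginPlay assigns a yellow minimap sprite before calling the parent.
; Tick makes it bob on a time-based sine wave and spin on all three axes.
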(event EventBeginPlay
  (Variables|Default|SetMinimapSprite "/Game/Assets/Textures/MiniMap/SPR_MapPowerup_Yellow.SPR_MapPowerup_Yellow")
  (|CallParentFunction))

(event Collision|EventActorBeginOverlap
  (params (OtherActor :type Actor%20Object%20Reference))
  (bind _asbp_player_character (Utilities|Casting|CastToBP_PlayerCharacter OtherActor))
  (Variables|/Script/SecondPersonShooter.PlayerCharacter|SetSuperWeaponTime _asbp_player_character 6.0)
  (Variables|/Script/SecondPersonShooter.PlayerCharacter|Setweapon _asbp_player_character "Laser")
  (Variables|/Script/SecondPersonShooter.PlayerCharacter|SetSuperWeaponSpeed _asbp_player_character 3.0)
  (Audio|PlaySoundatLocation "/Game/Assets/Audio/ammo-pick-up.ammo-pick-up" (Transformation|GetActorLocation))
  (Actor|DestroyActor))

(event EventTick
  (params (DeltaSeconds :type Float%20%28single-precision%29))
  (bind _returnvalue (Utilities|Time|GetWorldDeltaSeconds))
  (bind _returnvalue_2 (* _returnvalue 6e+01))
  (Transformation|AddWorldOffset (Variables|Default|GetDefaultSceneRoot) (Math|Vector|MakeVector 0.0 0.0 (* (Math|Trig|Sin(Radians) (* (Utilities|Time|GetGameTimeinSeconds) 2.0)) 0.2)) false false)
  (Transformation|AddLocalRotation (Variables|Default|GetDefaultSceneRoot) (Math|Rotator|MakeRotator _returnvalue_2 _returnvalue_2 _returnvalue_2) false false))

(fn ConstructionScript)