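; BP_PickUp is a pickup actor that shows itself on the game's minimap while it exists in the world.
; On BeginPlay it casts the game mode to BP_GameMode and registers itself with BPMiniMap using its MinimapSprite.
; On Destroyed it removes itself from the minimap through the same path.
; The file contains no collection or effect logic, and the construction script is empty.
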(event EventBeginPlay
  (Default|AddActortoMiniMap (Variables|/Game/Blueprints/BP_GameMode.BP_GameMode_C|GetBP_MiniMap (.AsBP%20Game%20Mode (Utilities|Casting|CastToBP_GameMode (Game|GetGameMode)))) self (Variables|Default|GetMinimapSprite)))

(event EventDestroyed
  (Default|RemoveActorfromMiniMap (Variables|/Game/Blueprints/BP_GameMode.BP_GameMode_C|GetBP_MiniMap (.AsBP%20Game%20Mode (Utilities|Casting|CastToBP_GameMode (Game|GetGameMode)))) self))

(fn ConstructionScript)