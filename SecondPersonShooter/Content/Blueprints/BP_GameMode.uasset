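; Game mode Blueprint that, in Horde Mode, periodically spawns power-up pickups while gameplay is running.
; Tick switches on the current mode, checks the running state, and fills the spawn point list from level TargetPoints when empty.
; A Delay on Tick paces spawning, after which a random fire rate or speed pickup spawns at a random point, ignoring collision.
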(event EventBeginPlay)

(event EventTick
  (params (DeltaSeconds :type Float%20%28single-precision%29))
  (switch Utilities|FlowControl|Switch|SwitchonEGameMode (Variables|Default|GetCurrentGameMode)
    (:HordeMode
      ;[1 1 1] Update Horde Mode
      (bind _asbp_game_mode (Utilities|Casting|CastToBP_GameMode (Game|GetGameMode)))
      (if (Class|DefaultGameMode|IsGameplayRunning _asbp_game_mode)
        (if (> (Utilities|Array|Length (Variables|Default|GetSpawnPoints)) 0)
          _
          (else
            (bind _outactors (Actor|GetAllActorsOfClass "/Script/Engine.TargetPoint"))
            (Variables|Default|SetSpawnPoints _outactors)))
        (Utilities|FlowControl|Delay 15.0)
        (switch int (Math|Random|RandomIntegerinRange 0 1)
          (:0
            (Game|SpawnActorfromClass "/Game/Blueprints/BP_FireRatePickup.BP_FireRatePickup_C" (Transformation|GetActorTransform (Utilities|Array|Get(acopy) (Variables|Default|GetSpawnPoints) (Math|Random|RandomIntegerinRange 0 (- (Utilities|Array|Length (Variables|Default|GetSpawnPoints)) 1)))) "AlwaysSpawn" 0 0))
          (:1
            (Game|SpawnActorfromClass "/Game/Blueprints/BP_SpeedPickup.BP_SpeedPickup_C" (Transformation|GetActorTransform (Utilities|Array|Get(acopy) (Variables|Default|GetSpawnPoints) (Math|Random|RandomIntegerinRange 0 (- (Utilities|Array|Length (Variables|Default|GetSpawnPoints)) 1)))) "AlwaysSpawn" 0 0)))))
    (:WaveMode)))

(fn ConstructionScript)