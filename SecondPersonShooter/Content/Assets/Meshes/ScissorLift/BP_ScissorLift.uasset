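; Scissor lift actor that builds a configurable stack of scissor segments and can animate raising and lowering.
; The construction script creates inner and outer instanced scissor meshes for the segment count, then applies the current height.
; A shared update function pitches the two sets in opposite directions, stacks them using a curve-driven offset, and seats the cage on the top segment.
; When Move is enabled, Tick drives the height with a clamped, time-based sine wave.
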(event EventBeginPlay)

(event Collision|EventActorBeginOverlap
  (params (OtherActor :type Actor%20Object%20Reference)))

(event EventTick
  (params (DeltaSeconds :type Float%20%28single-precision%29))
  (if (Variables|Default|GetMove)
    (Variables|Default|SetHeight (Math|Float|Clamp(Float) (- (* (Math|Float|Absolute(Float) (Math|Trig|Sin(Radians) (* (Utilities|Time|GetGameTimeinSeconds) (/ (Variables|Default|GetMoveSpeed) 3e+02)))) 1.5) 0.5) 0.0 0.5))
    (CallFunction|UpdateScissorLiftHeight)))

(fn ConstructionScript
  (Components|InstancedStaticMesh|ClearInstances (Variables|Default|GetInnerScissors))
  (for _index (range 0 (- (Variables|Default|GetScissorsNr) 1))
    (Components|InstancedStaticMesh|AddInstance (Variables|Default|GetInnerScissors) (Math|Transform|MakeTransform "0.0,0.0,0.0" "0.0,0.0,0" "1,1,1"))
    (Components|InstancedStaticMesh|AddInstance (Variables|Default|GetOuterScissors) (Math|Transform|MakeTransform "0.0,0.0,0.0" "0.0,0.0,0" "1,1,1")))
  (CallFunction|UpdateScissorLiftHeight))

(fn UpdateScissorLiftHeight
  (bind _height (Variables|Default|GetHeight))
  (Variables|Default|SetHeightOffset (Math|Curves|GetFloatValue (Variables|Default|GetOffsetCurve) (Variables|Default|GetHeight)))
  (Components|InstancedStaticMesh|UpdateInstanceTransform (Variables|Default|GetInnerScissors) 0 (Math|Transform|MakeTransform (Math|Vector|MakeVector 0.0 0.0 (/ (* (Variables|Default|GetHeightOffset) _height) 2.0)) (Math|Rotator|MakeRotator 0.0 (* _height 4e+01) 0.0) "1,1.000000,1.000000") false false)
  (Components|InstancedStaticMesh|UpdateInstanceTransform (Variables|Default|GetOuterScissors) 0 (Math|Transform|MakeTransform (Math|Vector|MakeVector 0.0 0.0 (/ (* (Variables|Default|GetHeightOffset) _height) 2.0)) (Math|Rotator|MakeRotator 0.0 (* (Variables|Default|GetHeight) -45.0) 0.0) "1,1,1.000000") false false)
  (for _index (range 1 (- (Variables|Default|GetScissorsNr) 1))
    (Components|InstancedStaticMesh|UpdateInstanceTransform (Variables|Default|GetInnerScissors) _index (Math|Transform|MakeTransform (Math|Vector|MakeVector 0.0 0.0 (+ (+ (* _index (Variables|Default|GetBaseOffset)) (/ (* (Variables|Default|GetHeightOffset) _height) 2.0)) (* (* _index (Variables|Default|GetHeightOffset)) (Variables|Default|GetHeight)))) (Math|Rotator|MakeRotator 0.0 (* (Variables|Default|GetHeight) 4e+01) 0.0) "1,1,1.000000") false false)
    (Components|InstancedStaticMesh|UpdateInstanceTransform (Variables|Default|GetOuterScissors) _index (Math|Transform|MakeTransform (Math|Vector|MakeVector 0.0 0.0 (+ (+ (* _index (Variables|Default|GetBaseOffset)) (/ (* (Variables|Default|GetHeightOffset) _height) 2.0)) (* (* _index (Variables|Default|GetHeightOffset)) (Variables|Default|GetHeight)))) (Math|Rotator|MakeRotator 0.0 (* (Variables|Default|GetHeight) -45.0) 0.0) "1,1,1.000000") false false))
  (Transformation|SetRelativeLocation (Variables|Default|GetScissorLift_Cage) (Math|Vector|MakeVector 0.0 0.0 (+ (.z (.location (.OutInstanceTransform (Components|InstancedStaticMesh|GetInstanceTransform (Variables|Default|GetInnerScissors) (- (Variables|Default|GetScissorsNr) 1) false)))) (/ (* (Variables|Default|GetHeightOffset) (Variables|Default|GetHeight)) 2.0))) false false)
  (return))