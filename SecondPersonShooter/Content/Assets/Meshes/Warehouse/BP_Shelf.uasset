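; BP_Shelf is a procedural warehouse shelving actor that builds a rack grid of configurable length and height, randomly stocked with crates.
; The construction script creates separate hierarchical instanced static mesh components for shelves and crates, then adds a shelf instance in each grid cell.
; Each shelf has three crate slots, each filled by a seeded random stream roll against CrateChance, making layouts repeatable per seed.
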(event EventBeginPlay)

(event Collision|EventActorBeginOverlap
  (params (OtherActor :type Actor%20Object%20Reference)))

(event EventTick
  (params (DeltaSeconds :type Float%20%28single-precision%29)))

(fn ConstructionScript
  (bind _random_streem (Variables|Default|GetRandom%20Streem))
  (bind _returnvalue (Math|Random|RandomFloatfromStream _random_streem))
  (bind _returnvalue_2 (AddComponent|AddHierarchicalInstancedStaticMeshComponent false))
  (bind _output_get (Variables|Default|SetCrateMeshes _returnvalue_2))
  (Components|StaticMesh|SetStaticMesh _output_get "/Game/Assets/Meshes/Warehouse/Crate.Crate")
  (bind _returnvalue_3 (AddComponent|AddHierarchicalInstancedStaticMeshComponent false))
  (bind _output_get_2 (Variables|Default|SetShelfMeshes _returnvalue_3))
  (Components|StaticMesh|SetStaticMesh _output_get_2 "/Game/Assets/Meshes/Warehouse/Shelf.Shelf")
  (Math|Random|SetRandomStreamSeed (Variables|Default|GetRandom%20Streem) (Variables|Public|GetInitalSeed))
  (for _index (range 0 (- (Variables|Public|GetLength) 1))
    (for _index_2 (range 0 (- (Variables|Public|GetHeight) 1))
      (Components|InstancedStaticMesh|AddInstance (Variables|Default|GetShelfMeshes) (Math|Transform|MakeTransform (Math|Vector|MakeVector 0.0 (* _index 3.8e+02) (* _index_2 1.9e+02)) "0, 0, 0" "1,1,1"))
      (if (<= _returnvalue (Variables|Public|GetCrateChance))
        (Components|InstancedStaticMesh|AddInstance (Variables|Default|GetCrateMeshes) (Math|Transform|MakeTransform (- (Math|Vector|MakeVector 0.0 (* _index 3.8e+02) (+ (* _index_2 1.9e+02) 3.0)) "0.000000,115.000000, 0") "0, 0, 0" "1,1,1")))
      (if (<= _returnvalue (Variables|Public|GetCrateChance))
        (Components|InstancedStaticMesh|AddInstance (Variables|Default|GetCrateMeshes) (Math|Transform|MakeTransform (+ (Math|Vector|MakeVector 0.0 (* _index 3.8e+02) (+ (* _index_2 1.9e+02) 3.0)) "0.000000,0.000000, 0") "0, 0,0.000000" "1,1.000000,1")))
      (if (<= _returnvalue (Variables|Public|GetCrateChance))
        (Components|InstancedStaticMesh|AddInstance (Variables|Default|GetCrateMeshes) (Math|Transform|MakeTransform (+ (Math|Vector|MakeVector 0.0 (* _index 3.8e+02) (+ (* _index_2 1.9e+02) 3.0)) "0,115.000000, 0") "0, 0, 0" "1,1,1"))))))